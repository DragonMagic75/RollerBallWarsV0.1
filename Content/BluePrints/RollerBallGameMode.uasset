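; RollerBall game mode that creates local players from the game instance's player count and handles their spawning and respawning.
; SpawnPlayer replaces the controller's pawn at the first unoccupied spawn point, assigns a random material saved by controller ID and disables input.
; ReSpawnPlayer replaces the pawn at a spawn point via PlayerSpawnPoint, keeping score and material, clearing land mines and enabling gravity.
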(event Custom|Spawn%20Player
  (params (PlayerControler :type Player%20Controller%20Object%20Reference))
  (bind _returnvalue (Pawn|GetControlledPawn PlayerControler))
  ;[1 1 1] Spawn Player andy Set Player Material
  (Utilities|IsValid _returnvalue
    (:Is%20Valid
      (Actor|DestroyActor _returnvalue)
      (bind _returnvalue_2 (Class|GameplayStatics|GetPlayerControllerID PlayerControler))
      (bind _outactors (Actor|GetAllActorsOfClass "/Game/BluePrints/PlayerSpawnPoints.PlayerSpawnPoints_C"))
      (bind _array_element (Utilities|Array|ForEachLoopwithBreak _outactors :!label _label)
        (:LoopBody
          (if (not (Variables|/Game/BluePrints/PlayerSpawnPoints.PlayerSpawnPoints_C|GetIsOccupied _array_element))
            (Variables|/Game/BluePrints/PlayerSpawnPoints.PlayerSpawnPoints_C|SetIsOccupied _array_element true)
            (bind _playermaterial (CallFunction|SetMaterial _returnvalue_2))
            (Utilities|Array|Insert (Variables|Default|GetMaterial) _playermaterial _returnvalue_2)
            (Development|PrintString (Utilities|String|ToString(Integer) _returnvalue_2))
            (bind _returnvalue_3 (Game|SpawnActorfromClass "/Game/BluePrints/PlayerBlueprint.PlayerBlueprint_C" (Transformation|GetActorTransform _array_element) "Undefined" 0 _returnvalue_2 0 0 _playermaterial))
            (Pawn|Possess PlayerControler _returnvalue_3)
            (Input|DisableInput _returnvalue_3 PlayerControler)
            (goto _label Break)))))))

(event Custom|ReSpawn%20Player
  (params (PlayerController :type Player%20Controller%20Object%20Reference) (Score :type Integer))
  (bind _returnvalue (Pawn|GetControlledPawn PlayerController))
  ;[1 1 1] ReSpawn Player
  (Utilities|IsValid _returnvalue
    (:Is%20Valid
      (Actor|DestroyActor _returnvalue)
      (bind _returnvalue_2 (Class|GameplayStatics|GetPlayerControllerID PlayerController))
      (bind _outactors (Actor|GetAllActorsOfClass "/Game/BluePrints/PlayerSpawnPoints.PlayerSpawnPoints_C"))
      (Variables|Default|SetPlayerSpawnPoints _outactors)
      (bind _returnvalue_3 (Game|SpawnActorfromClass "/Game/BluePrints/PlayerBlueprint.PlayerBlueprint_C" (Utilities|PlayerSpawnPoint) "Undefined" 0 _returnvalue_2 Score 0 (Utilities|Array|Get(acopy) (Variables|Default|GetMaterial) _returnvalue_2)))
      (Default|EnableGravity _returnvalue_3)
      (Pawn|Possess PlayerController _returnvalue_3))))

(event EventBeginPlay
  ;[1 1 1] Spawn Player andy Set Player Material
  (Utilities|FlowControl|DoN 1
    (:Exit
      (bind _asroller_ball_instance (Utilities|Casting|CastToRollerBallInstance (Game|GetGameInstance)))
      (for _index (range 0 (- (Variables|/Game/BluePrints/RollerBallInstance.RollerBallInstance_C|GetPlayerCount _asroller_ball_instance) 1))
        (Class|GameplayStatics|CreatePlayer -1)))))

(fn ConstructionScript)

(fn SetMaterial
  (params (PlayerID :type Integer))
  (bind _playermaterial (Variables|Default|GetPlayerMaterial))
  ;[1 1 1] Sets the Player Material
  (return (Utilities|Array|Get(acopy) _playermaterial (Math|Random|RandomIntegerinRange 0 (- (Utilities|Array|Length _playermaterial) 1)))))