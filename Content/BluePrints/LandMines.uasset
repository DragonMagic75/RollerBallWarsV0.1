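; Land mine actor that damages any player other than its owner who overlaps it.
; Overlap events on the mine are enabled shortly after BeginPlay.
; On a hit it damages the victim, credits score to the owning player, plays a sound and particle at the victim's location, then destroys itself.
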(event EventBeginPlay
  (Utilities|FlowControl|Delay 0.2)
  (Variables|/Script/Engine.PrimitiveComponent|SetbGenerateOverlapEvents (Variables|Default|GetLandMine) true))

(event Collision|EventActorBeginOverlap
  (params (OtherActor :type Actor%20Object%20Reference))
  (bind _returnvalue (Transformation|GetActorLocation OtherActor))
  (if (!= (Components|GetOwner) OtherActor)
    (bind _asplayer_blueprint (Utilities|Casting|CastToPlayerBlueprint OtherActor))
    (Default|Damage _asplayer_blueprint (Variables|Default|GetLandMineDamage))
    (bind _asplayer_blueprint_2 (Utilities|Casting|CastToPlayerBlueprint (Components|GetOwner)))
    (Default|PlayerScore _asplayer_blueprint_2)
    (Audio|PlaySoundatLocation (Variables|Default|GetHitSound) _returnvalue)
    (Effects|SpawnEmitteratLocation (Variables|Default|GetHit%20Particle) _returnvalue)
    (Actor|DestroyActor)))

(fn ConstructionScript)