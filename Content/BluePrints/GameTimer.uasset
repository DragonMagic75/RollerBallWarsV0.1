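; GameTimer is an actor Blueprint that counts down the match clock stored in RollerBallInstance.
; Each Tick it looks up the MatchStart widget and proceeds only once that widget's MatchTimer reaches zero.
; A one-second Delay on Tick throttles the countdown, subtracting one from the game instance's GameTimer per pass and clamping it at zero.
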(event EventBeginPlay)

(event Collision|EventActorBeginOverlap
  (params (OtherActor :type Actor%20Object%20Reference)))

(event EventTick
  (params (DeltaSeconds :type Float%20%28single-precision%29))
  (bind _foundwidgets (Widget|GetAllWidgetsOfClass "/Game/BluePrints/UIElements/MatchStart.MatchStart_C" true))
  (if (== (Variables|/Game/BluePrints/UIElements/MatchStart.MatchStart_C|GetMatchTimer (Utilities|Array|Get(acopy) _foundwidgets)) 0.0)
    (Utilities|FlowControl|Delay 1.0)
    (bind _asroller_ball_instance (Utilities|Casting|CastToRollerBallInstance (Game|GetGameInstance)))
    (Variables|/Game/BluePrints/RollerBallInstance.RollerBallInstance_C|SetGameTimer _asroller_ball_instance (- (Variables|/Game/BluePrints/RollerBallInstance.RollerBallInstance_C|GetGameTimer _asroller_ball_instance) 1.0))
    (if (< (Variables|/Game/BluePrints/RollerBallInstance.RollerBallInstance_C|GetGameTimer _asroller_ball_instance) 5.0)
      (if (<= (Variables|/Game/BluePrints/RollerBallInstance.RollerBallInstance_C|GetGameTimer _asroller_ball_instance) 0.0)
        (Variables|/Game/BluePrints/RollerBallInstance.RollerBallInstance_C|SetGameTimer _asroller_ball_instance 0.0)))))

(fn ConstructionScript)