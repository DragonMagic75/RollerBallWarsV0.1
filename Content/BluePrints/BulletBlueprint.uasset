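; Bullet projectile actor that damages players, credits its shooter and destroys itself on impact or after a short Tick-driven delay.
; On Hit, a Sequence first damages a struck player and, if the owner is a player, awards score and plays hit effects.
; It then plays sound and environment particles for every hit, player hits included.
; Finally, hits on the Arena apply damage and impulse to its destructible glass mesh.
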(event EventTick
  (params (DeltaSeconds :type Float%20%28single-precision%29))
  (Utilities|FlowControl|Delay 3.0)
  (Actor|DestroyActor))

(event Collision|EventHit
  (params (MyComp :type Primitive%20Component%20Object%20Reference) (Other :type Actor%20Object%20Reference) (OtherComp :type Primitive%20Component%20Object%20Reference) (bSelfMoved :type Boolean) (HitLocation :type Vector) (HitNormal :type Vector) (NormalImpulse :type Vector :default "0, 0, 0") (Hit :type Hit%20Result%20Structure%20%28by%20ref%29))
  ;[1 1 1] Default Bullet Hit
  (Utilities|FlowControl|Sequence
    (:then_0
      (bind _asplayer_blueprint (Utilities|Casting|CastToPlayerBlueprint Other))
      (Default|Damage _asplayer_blueprint (Variables|Default|GetBulletDamage))
      (bind _asplayer_blueprint_2 (Utilities|Casting|CastToPlayerBlueprint (Components|GetOwner)))
      (Utilities|IsValid _asplayer_blueprint_2
        (:Is%20Valid
          (Default|PlayerScore _asplayer_blueprint_2))
        (:Is%20Not%20Valid
          _))
      (Actor|DestroyActor)
      (Audio|PlaySoundatLocation (Variables|Default|GetHitSound) HitLocation)
      (Effects|SpawnEmitteratLocation (Variables|Default|GetHitParticle) HitLocation))
    (:then_1
      (Actor|DestroyActor)
      (Audio|PlaySoundatLocation (Variables|Default|GetHitSound) HitLocation)
      (Effects|SpawnEmitteratLocation (Variables|Default|GetEnvironmentParticle) HitLocation))
    (:then_2
      (bind _asarena (Utilities|Casting|CastToArena Other))
      (Utilities|IsValid (Variables|/Game/BluePrints/Arena.Arena_C|GetSM_NexusArena_Glass_DM _asarena)
        (:Is%20Valid
          (Game|Damage|ApplyDamage (Variables|/Game/BluePrints/Arena.Arena_C|GetSM_NexusArena_Glass_DM _asarena) 0.5 HitLocation HitNormal 0.0))))))

(fn ConstructionScript)