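; Player controller for the RollerBall game that handles joining a match and pausing.
; The 1 key or gamepad Special Right runs once, asking RollerBallGameMode to spawn this player and notifying top-level MatchStart widgets through PlayerStart.
; Escape or gamepad Special Left drives a FlipFlop that alternately pauses and unpauses the game.
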(event EventBeginPlay)

(event Input|KeyboardEvents|Escape
  (params (Key :type Key%20Structure :default "AnyKey"))
  ;[1 1 1] Pause Game
  (:Pressed
    (Utilities|FlowControl|FlipFlop
      (:A
        (Game|SetGamePaused true))
      (:B
        (Game|SetGamePaused false)))))

(event Input|GamepadEvents|GamepadSpecialRight
  (params (Key :type Key%20Structure :default "AnyKey"))
  (bind _self self)
  ;[1 1 1] Spawn Player Controler
  (:Pressed
    (Utilities|FlowControl|DoN 1
      (:Exit
        (bind _asroller_ball_game_mode (Utilities|Casting|CastToRollerBallGameMode (Game|GetGameMode)))
        (Default|SpawnPlayer _asroller_ball_game_mode _self)
        (bind _foundwidgets (Widget|GetAllWidgetsOfClass "/Game/BluePrints/UIElements/MatchStart.MatchStart_C" true))
        (Default|PlayerStart _foundwidgets _self)))))

(event Input|KeyboardEvents|1
  (params (Key :type Key%20Structure :default "AnyKey"))
  (bind _self self)
  ;[1 1 1] Spawn Player Controler
  (:Pressed
    (Utilities|FlowControl|DoN 1
      (:Exit
        (bind _asroller_ball_game_mode (Utilities|Casting|CastToRollerBallGameMode (Game|GetGameMode)))
        (Default|SpawnPlayer _asroller_ball_game_mode _self)
        (bind _foundwidgets (Widget|GetAllWidgetsOfClass "/Game/BluePrints/UIElements/MatchStart.MatchStart_C" true))
        (Default|PlayerStart _foundwidgets _self)))))

(event Input|GamepadEvents|GamepadSpecialLeft
  (params (Key :type Key%20Structure :default "AnyKey"))
  ;[1 1 1] Pause Game
  (:Pressed
    (Utilities|FlowControl|FlipFlop
      (:A
        (Game|SetGamePaused true))
      (:B
        (Game|SetGamePaused false)))))

(fn ConstructionScript)