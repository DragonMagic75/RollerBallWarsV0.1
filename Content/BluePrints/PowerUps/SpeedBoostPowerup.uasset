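; Speed boost pickup actor that grants the player a speed boost power-up on overlap.
; When a PlayerBlueprint overlaps the SpeedPowerUp component, it sets that player's power-up text and SpeedBoostPowerUp flag, then destroys itself.
; The construction script creates a dynamic material instance and applies it to the pickup component.
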(event OnComponentBeginOverlap(SpeedPowerUp)
  (params (OverlappedComponent :type Primitive%20Component%20Object%20Reference) (OtherActor :type Actor%20Object%20Reference) (OtherComp :type Primitive%20Component%20Object%20Reference) (OtherBodyIndex :type Integer) (bFromSweep :type Boolean) (SweepResult :type Hit%20Result%20Structure%20%28by%20ref%29))
  (bind _output_get (Variables|Default|SetOverlappingActor OtherActor))
  (bind _asplayer_blueprint (Utilities|Casting|CastToPlayerBlueprint _output_get))
  (Variables|/Game/BluePrints/PlayerBlueprint.PlayerBlueprint_C|SetPowerUpText _asplayer_blueprint "SpeedBoost")
  (Variables|/Game/BluePrints/PlayerBlueprint.PlayerBlueprint_C|SetSpeedBoostPowerUp _asplayer_blueprint true)
  (Actor|DestroyActor))

(fn ConstructionScript
  (bind _returnvalue (Rendering|Material|CreateDynamicMaterialInstance "/Game/Material/Player.Player" :!class /Script/Engine.KismetMaterialLibrary))
  (Variables|Default|SetSpeedBoostMaterial _returnvalue)
  (Rendering|Material|SetMaterial (Variables|Default|GetSpeedPowerUp) 0 (Variables|Default|GetSpeedBoostMaterial)))