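; Pickup actor that grants the player invulnerability in the roller-ball game.
; On overlap with a PlayerBlueprint lacking the power-up, it sets the invulnerability flag and power-up text, increments the game instance's pickup counter and destroys itself.
; The construction script creates a dynamic instance of the Ring material and applies it to the pickup's InvulnerablePowerUp component.
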(event OnComponentBeginOverlap(InvulnerablePowerUp)
  (params (OverlappedComponent :type Primitive%20Component%20Object%20Reference) (OtherActor :type Actor%20Object%20Reference) (OtherComp :type Primitive%20Component%20Object%20Reference) (OtherBodyIndex :type Integer) (bFromSweep :type Boolean) (SweepResult :type Hit%20Result%20Structure%20%28by%20ref%29))
  (bind _output_get (Variables|Default|SetOverlapping%20Actor OtherActor))
  (bind _asplayer_blueprint (Utilities|Casting|CastToPlayerBlueprint _output_get))
  (if (not (Math|Boolean|Equal(Boolean) (Variables|/Game/BluePrints/PlayerBlueprint.PlayerBlueprint_C|GetInvulnerable%20PowerUp _asplayer_blueprint) true))
    (bind _asroller_ball_instance (Utilities|Casting|CastToRollerBallInstance (Game|GetGameInstance)))
    (Variables|/Game/BluePrints/PlayerBlueprint.PlayerBlueprint_C|SetInvulnerable%20PowerUp _asplayer_blueprint true)
    (Variables|/Game/BluePrints/PlayerBlueprint.PlayerBlueprint_C|SetPowerUpText _asplayer_blueprint "Invulnerable")
    (Variables|/Game/BluePrints/RollerBallInstance.RollerBallInstance_C|SetIPowerUPCount _asroller_ball_instance (+ (Variables|/Game/BluePrints/RollerBallInstance.RollerBallInstance_C|GetIPowerUPCount _asroller_ball_instance) 1))
    (Actor|DestroyActor)))

(fn ConstructionScript
  (bind _returnvalue (Rendering|Material|CreateDynamicMaterialInstance "/Game/Material/Chair/Ring.Ring" :!class /Script/Engine.KismetMaterialLibrary))
  (Variables|Default|SetInvulnerabilityMat _returnvalue)
  (Rendering|Material|SetMaterial (Variables|Default|GetInvulnerablePowerUp) 0 (Variables|Default|GetInvulnerabilityMat)))