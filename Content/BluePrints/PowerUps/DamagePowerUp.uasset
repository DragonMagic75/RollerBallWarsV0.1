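; Damage power-up pickup that grants the player a damage boost flag when touched.
; On overlap with a PlayerBlueprint lacking the power-up, it sets the flag and pickup text, increments the damage power-up count in RollerBallInstance, then destroys itself.
; A player who already holds the power-up leaves the pickup in place.
; The construction script applies a dynamic material instance created from EnemyMaterial to the mesh.
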(event OnComponentBeginOverlap(DamagePowerUp)
  (params (OverlappedComponent :type Primitive%20Component%20Object%20Reference) (OtherActor :type Actor%20Object%20Reference) (OtherComp :type Primitive%20Component%20Object%20Reference) (OtherBodyIndex :type Integer) (bFromSweep :type Boolean) (SweepResult :type Hit%20Result%20Structure%20%28by%20ref%29))
  (bind _asplayer_blueprint (Utilities|Casting|CastToPlayerBlueprint OtherActor))
  (if (not (Math|Boolean|Equal(Boolean) (Variables|/Game/BluePrints/PlayerBlueprint.PlayerBlueprint_C|GetDamagePowerUp _asplayer_blueprint) true))
    (bind _asroller_ball_instance (Utilities|Casting|CastToRollerBallInstance (Game|GetGameInstance)))
    (Variables|/Game/BluePrints/PlayerBlueprint.PlayerBlueprint_C|SetDamagePowerUp _asplayer_blueprint true)
    (Variables|/Game/BluePrints/PlayerBlueprint.PlayerBlueprint_C|SetPowerUpText _asplayer_blueprint "Power Up")
    (Variables|/Game/BluePrints/RollerBallInstance.RollerBallInstance_C|SetDPowerUp%20Count _asroller_ball_instance (+ (Variables|/Game/BluePrints/RollerBallInstance.RollerBallInstance_C|GetDPowerUp%20Count _asroller_ball_instance) 1))
    (Actor|DestroyActor)))

(fn ConstructionScript
  (bind _returnvalue (Rendering|Material|CreateDynamicMaterialInstance "/Game/Material/EnemyMaterial.EnemyMaterial" :!class /Script/Engine.KismetMaterialLibrary))
  (Variables|Default|SetDamagePowerUpMat _returnvalue)
  (Rendering|Material|SetMaterial (Variables|Default|GetDamagePowerUp) 0 (Variables|Default|GetDamagePowerUpMat)))