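; AmmoManager spawns ion cannon, minigun and grenade ammo boxes after BeginPlay, each type after its own delay and in a configured count.
; Each spawn loop gathers all AmmoSpawnPoints, flags the first match as occupied and spawns at AmmoRandomPoint's transform, independent of the flagged point.
; Only grenades match free points; ion cannon and minigun match occupied ones.
; AmmoRandomPoint contains a random-point lookup, but that expression is unused.
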(event EventBeginPlay
  (Utilities|FlowControl|Sequence
    (:then_0
      (Utilities|FlowControl|Delay 5.0)
      (for _index (range 0 (- (Variables|Default|GetLaserAmmoBox) 1))
        (bind _outactors (Actor|GetAllActorsOfClass "/Game/BluePrints/Ammo/AmmoSpawnPoints.AmmoSpawnPoints_C"))
        (bind _output_get (Variables|Default|SetAmmoSpawnPoints _outactors))
        (bind _array_element (Utilities|Array|ForEachLoopwithBreak _output_get :!label _label)
          (:LoopBody
            (if (Variables|/Game/BluePrints/Ammo/AmmoSpawnPoints.AmmoSpawnPoints_C|GetIsOccupied _array_element)
              (Variables|/Game/BluePrints/Ammo/AmmoSpawnPoints.AmmoSpawnPoints_C|SetIsOccupied _array_element true)
              (Game|SpawnActorfromClass "/Game/BluePrints/Ammo/IonCannonAmmoBox.IonCannonAmmoBox_C" (Utilities|AmmoRandomPoint) "Undefined" 0 0)
              (goto _label Break))))))
    (:then_1
      (Utilities|FlowControl|Delay 1e+01)
      (for _index_2 (range 0 (- (Variables|Default|GetMiniGunAmmoBox) 1))
        (bind _outactors_2 (Actor|GetAllActorsOfClass "/Game/BluePrints/Ammo/AmmoSpawnPoints.AmmoSpawnPoints_C"))
        (bind _output_get_2 (Variables|Default|SetAmmoSpawnPoints _outactors_2))
        (bind _array_element_2 (Utilities|Array|ForEachLoopwithBreak _output_get_2 :!label _label_2)
          (:LoopBody
            (if (Variables|/Game/BluePrints/Ammo/AmmoSpawnPoints.AmmoSpawnPoints_C|GetIsOccupied _array_element_2)
              (Variables|/Game/BluePrints/Ammo/AmmoSpawnPoints.AmmoSpawnPoints_C|SetIsOccupied _array_element_2 true)
              (Game|SpawnActorfromClass "/Game/BluePrints/Ammo/MiniGunAmmoBox.MiniGunAmmoBox_C" (Utilities|AmmoRandomPoint) "Undefined" 0 0)
              (goto _label_2 Break))))))
    (:then_2
      (Utilities|FlowControl|Delay 7.0)
      (for _index_3 (range 0 (- (Variables|Default|GetGrenadeAmmoBox) 1))
        (bind _outactors_3 (Actor|GetAllActorsOfClass "/Game/BluePrints/Ammo/AmmoSpawnPoints.AmmoSpawnPoints_C"))
        (bind _output_get_3 (Variables|Default|SetAmmoSpawnPoints _outactors_3))
        (bind _array_element_3 (Utilities|Array|ForEachLoopwithBreak _output_get_3 :!label _label_3)
          (:LoopBody
            (if (not (Variables|/Game/BluePrints/Ammo/AmmoSpawnPoints.AmmoSpawnPoints_C|GetIsOccupied _array_element_3))
              (Variables|/Game/BluePrints/Ammo/AmmoSpawnPoints.AmmoSpawnPoints_C|SetIsOccupied _array_element_3 true)
              (Game|SpawnActorfromClass "/Game/BluePrints/Ammo/GrenadeAmmoBox.GrenadeAmmoBox_C" (Utilities|AmmoRandomPoint) "Undefined" 0 0)
              (goto _label_3 Break))))))))

(event EventTick
  (params (DeltaSeconds :type Float%20%28single-precision%29)))

(fn ConstructionScript)